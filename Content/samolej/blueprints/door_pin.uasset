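; Door actor with a PIN keypad that controls its locked state.
; On BeginPlay it gets the KeyPan widget from its widget component, stores it and binds a handler to its CodeEntered event.
; CheckCode compares the entered code with CorrectCode, unlocks on a match or locks otherwise, then clears the keypad's current code.
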(event EventBeginPlay
  (bind _askey_pan (Utilities|Casting|CastToKeyPan (UserInterface|GetUserWidgetObject (Variables|Default|GetWidget))))
  (bind _output_get (Variables|Default|SetkeypadUI _askey_pan))
  (EventDispatchers|BindEventtoCodeEntered _output_get (EventDispatchers|CreateEvent :!event CheckCode)))

(event Collision|EventActorBeginOverlap
  (params (OtherActor :type Actor%20Object%20Reference)))

(event EventTick
  (params (DeltaSeconds :type Float%20%28single-precision%29)))

(fn ConstructionScript
  (|CallParentFunction))

(fn CheckCode
  (params (codeEntered :type String) (keypadUI :type Key%20Pan%20Object%20Reference))
  (if (Utilities|Enum|Equal(Enum) codeEntered (Variables|Default|GetcorrectCode))
    (Variables|Default|SetisLocked false)
    (else
      (Variables|Default|SetisLocked true)))
  (Variables|/Game/samolej/widgets/KeyPan.KeyPan_C|SetCurrentCode (Variables|Default|GetkeypadUI) ""))