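; Player controller for a chess game that forwards mouse clicks to the chess board.
; On BeginPlay it shows the cursor and caches the first ChessBoard actor found in the level.
; Releasing the left mouse button traces under the cursor on the Visibility channel and passes the hit location to the board's click function, leaving all handling to the board.
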(event EventBeginPlay
  (Variables|Default|SetbShowMouseCursor true)
  (bind _outactors (Actor|GetAllActorsOfClass "/Game/samolej/chess/ChessBoard.ChessBoard_C"))
  (bind _aschess_board (Utilities|Casting|CastToChessBoard (Utilities|Array|Get(acopy) _outactors)))
  (Variables|Default|Setchessboard (Utilities|Array|MakeArray _aschess_board)))

(event EventTick
  (params (DeltaSeconds :type Float%20%28single-precision%29)))

(event Input|MouseEvents|LeftMouseButton
  (params (Key :type Key%20Structure :default "None"))
  (:Released
    (Default|CLick (Variables|Default|Getchessboard) (.Location (Collision|BreakHitResult (.HitResult (Game|Player|GetHitResultUnderCursorbyChannel "TraceTypeQuery1" true)))))))

(fn ConstructionScript)