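; Locked door actor that the adam character opens with E when holding a key, with a timeline driving the door's yaw.
; Separate overlap boxes toggle actor input, cache the character for the HasKey check, and show or remove a press-E widget.
; Leaving the cache box reverses the timeline, while pressing E again only resets the DoorClosed flag.
; A second E binding adds an audio component, and the interact action briefly pulses IsPressed.
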(event OnComponentBeginOverlap(Box)
  (params (OverlappedComponent :type Primitive%20Component%20Object%20Reference) (OtherActor :type Actor%20Object%20Reference) (OtherComp :type Primitive%20Component%20Object%20Reference) (OtherBodyIndex :type Integer) (bFromSweep :type Boolean) (SweepResult :type Hit%20Result%20Structure%20%28by%20ref%29))
  (bind _asadam (Utilities|Casting|CastToadam OtherActor)))

(event OnComponentEndOverlap(box_0)
  (params (OverlappedComponent :type Primitive%20Component%20Object%20Reference) (OtherActor :type Actor%20Object%20Reference) (OtherComp :type Primitive%20Component%20Object%20Reference) (OtherBodyIndex :type Integer))
  ;[1 1 1] Enable/Disable Input
  (Input|DisableInput (Game|GetPlayerController 0)))

(event OnComponentBeginOverlap(box_0)
  (params (OverlappedComponent :type Primitive%20Component%20Object%20Reference) (OtherActor :type Actor%20Object%20Reference) (OtherComp :type Primitive%20Component%20Object%20Reference) (OtherBodyIndex :type Integer) (bFromSweep :type Boolean) (SweepResult :type Hit%20Result%20Structure%20%28by%20ref%29))
  ;[1 1 1] Enable/Disable Input
  (Input|EnableInput (Game|GetPlayerController 0)))

(event OnComponentEndOverlap(Box)
  (params (OverlappedComponent :type Primitive%20Component%20Object%20Reference) (OtherActor :type Actor%20Object%20Reference) (OtherComp :type Primitive%20Component%20Object%20Reference) (OtherBodyIndex :type Integer))
  (Utilities|Casting|CastToadam OtherActor)
  (bind _doortimer (Timeline|Timeline_0 Reverse)
    (:Update
      (Transformation|SetRelativeRotation (Variables|Default|GetDoor) (Math|Rotator|MakeRotator 0.0 0.0 _doortimer) false false))))

(event OnComponentBeginOverlap(boxWBP)
  (params (OverlappedComponent :type Primitive%20Component%20Object%20Reference) (OtherActor :type Actor%20Object%20Reference) (OtherComp :type Primitive%20Component%20Object%20Reference) (OtherBodyIndex :type Integer) (bFromSweep :type Boolean) (SweepResult :type Hit%20Result%20Structure%20%28by%20ref%29))
  (Utilities|Casting|CastToadam OtherActor)
  (bind _returnvalue (UserInterface|CreateWidget "/Game/samolej/blueprints/WBP-pressE.WBP-pressE_C"))
  (UserInterface|Viewport|AddtoViewport _returnvalue 0))

(event OnComponentEndOverlap(boxWBP)
  (params (OverlappedComponent :type Primitive%20Component%20Object%20Reference) (OtherActor :type Actor%20Object%20Reference) (OtherComp :type Primitive%20Component%20Object%20Reference) (OtherBodyIndex :type Integer))
  (Utilities|Casting|CastToadam OtherActor)
  (Widget|RemovefromParent (stale OnComponentBeginOverlap(boxWBP) _returnvalue)))

(event Input|ActionEvents|InputActioninteract
  (params (Key :type Key%20Structure :default "None"))
  (:Pressed
    (Variables|Default|SetIsPressed? true)
    (Utilities|FlowControl|Delay 0.4)
    (Variables|Default|SetIsPressed? false)))

(event Input|KeyboardEvents|E
  (params (Key :type Key%20Structure :default "None"))
  (:Pressed
    (AddComponent|AddAudioComponent false)))

(event Input|KeyboardEvents|E
  (params (Key :type Key%20Structure :default "None"))
  (:Pressed
    (if (Variables|/Game/samolej/blueprints/adam.adam_C|GethasKey? (stale OnComponentBeginOverlap(Box) _asadam))
      (if (Variables|Default|GetDoorClosed)
        (Variables|Default|SetDoorClosed false)
        (bind _doortimer (Timeline|Timeline_0 Play)
          (:Update
            (Transformation|SetRelativeRotation (Variables|Default|GetDoor) (Math|Rotator|MakeRotator 0.0 0.0 _doortimer) false false)))
        (else
          (Variables|Default|SetDoorClosed true))))))

(fn ConstructionScript)